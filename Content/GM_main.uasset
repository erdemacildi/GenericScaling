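; Game mode that sets up a scene and randomly rescales a tagged actor at timed intervals.
; BeginPlay switches the view to the MainCam-tagged camera, adds the HUD, caches the wantToScale actor's default scale and applies a material.
; Tick uses a near-equal time check to multiply or divide each default axis by random factors.
; Movie render queue and Houdini asset logic is present but never runs.
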(event `self.ReceiveBeginPlay`
  (`self.Set Cam`)
  (`self.Set HUD`)
  (`self.GetActorAndDefaultSize`)
  (`self.SetActorMetarial`))

(event `self.ReceiveTick`
  (params (DeltaSeconds :type "Float (single-precision)"))
  (`self.Rescale Actor`)
  (if (`KismetMathLibrary.NearlyEqual_FloatFloat` (`GameplayStatics.GetTimeSeconds`) (+ (`self.RenderTime`) 0.5) 0.1)
    _))

(fn `CreatingRandomVector`
  (bind _returnvalue (`KismetMathLibrary.RandomFloatInRange` 1.0 5.0))
  (bind _returnvalue_2 (`KismetMathLibrary.RandomFloatInRange` 1.0 5.0))
  (bind _returnvalue_3 (`KismetMathLibrary.RandomFloatInRange` 1.0 5.0))
  (bind (_defaultactorscale_x _defaultactorscale_y _defaultactorscale_z) (`KismetMathLibrary.BreakVector` (`self.DefaultActorScale`)))
  (bind (_defaultactorscale_x_2 _defaultactorscale_y_2 _defaultactorscale_z_2) (`KismetMathLibrary.BreakVector` (`self.DefaultActorScale`)))
  (if (`KismetMathLibrary.RandomBool`)
    (set `self.randomVector` (`KismetMathLibrary.MakeVector` (* _defaultactorscale_x_2 _returnvalue) (* _defaultactorscale_y_2 _returnvalue_2) (* _defaultactorscale_z_2 _returnvalue_3)))
    (else
      (set `self.randomVector` (`KismetMathLibrary.MakeVector` (/ _defaultactorscale_x _returnvalue) (/ _defaultactorscale_y _returnvalue_2) (/ _defaultactorscale_z _returnvalue_3)))))
  (`self.SetActorScale3D` (`self.MainActor`) (`self.randomVector`)))

(fn `GetActorAndDefaultSize`
  (bind _outactors (`GameplayStatics.GetAllActorsOfClass` "/Game/BP_Actor.BP_Actor_C"))
  (for _array_element _outactors
    (if (`self.ActorHasTag` _array_element "wantToScale")
      (bind _output_get (set `self.MainActor` _array_element))
      (bind (_returnvalue_x _returnvalue_y _returnvalue_z) (`KismetMathLibrary.BreakVector` (`self.GetActorScale3D` _output_get)))
      (set `self.DefaultActorScale` (`KismetMathLibrary.MakeVector` _returnvalue_x _returnvalue_y _returnvalue_z)))))

(fn `NewFunction_0`)

(fn `Rescale Actor`
  (if (`KismetMathLibrary.NearlyEqual_FloatFloat` (`self.NextScaleTime`) (`GameplayStatics.GetTimeSeconds`) 0.1)
    (set `self.NextScaleTime` (+ (`self.NextScaleTime`) (`self.ScaleTimeGap`)))
    (`self.CreatingRandomVector`)))

(fn `Set Cam`
  (bind _outactors (`GameplayStatics.GetAllActorsOfClass` "/Game/BP_cam.BP_cam_C"))
  (for _array_element _outactors
    (if (`self.ActorHasTag` _array_element "MainCam")
      (bind _output_get (set `self.MainCam` _array_element))
      (`PlayerController.SetViewTargetWithBlend` (`GameplayStatics.GetPlayerController` 0) _output_get 0.0 "VTBlend_Linear" 0.0 false))))

(fn `Set HUD`
  (bind _returnvalue (`|CreateWidget` "/Game/HUD.HUD_C"))
  (`UserWidget.AddToViewport` _returnvalue 0))

(fn `SetActorMetarial`
  (`PrimitiveComponent.SetMaterial` (`self.GetComponentByClass` (`self.MainActor`) "/Script/Engine.PrimitiveComponent") 0 "/Game/MainMaterial.MainMaterial"))

(fn `UserConstructionScript`)