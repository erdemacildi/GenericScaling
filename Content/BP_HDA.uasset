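; BP_HDA is an actor Blueprint that appears to be a scratch test for the Houdini Engine plugin, built around a Houdini component named Test.
; Its only live logic prints the actor's X scale on BeginPlay; Tick, the construction script and NewFunction_0 do nothing.
; Disconnected nodes hold experiments with listing child components, casting to Houdini component types, setting HDA parameters and adding handle components.
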(event `self.ReceiveBeginPlay`
  (bind _returnvalue_x (`KismetMathLibrary.BreakVector` (`self.GetActorScale3D`)))
  (`KismetSystemLibrary.PrintString` (`KismetStringLibrary.Conv_DoubleToString` _returnvalue_x)))

(fn `NewFunction_0`)

(fn `UserConstructionScript`)